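; BP_GlassVideoPanel is a submenu Blueprint for a glass panel that plays a video alongside separate audio.
; BeginPlay starts Video and Audio together.
; Tick polls both: while the video plays, stopped audio restarts from zero with a debug print, and when the video is not playing it calls Pause on the video, leaving audio untouched.
; The construction script only calls its parent.
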(event `self.ReceiveBeginPlay`
  (`parent.ReceiveBeginPlay`)
  (`MediaPlayer.Play` (`self.video`))
  (`AudioComponent.Play` (`self.Audio`) 0.0))

(event `self.ReceiveTick`
  (params (DeltaSeconds :type "Float (single-precision)"))
  (bind _returnvalue (`AudioComponent.IsPlaying` (`self.Audio`)))
  (`parent.ReceiveTick` 0.0)
  (if (`MediaPlayer.IsPlaying` (`self.video`))
    (if (not _returnvalue)
      (`KismetSystemLibrary.PrintString` (`KismetStringLibrary.Conv_BoolToString` _returnvalue))
      (`AudioComponent.Play` (`self.Audio`) 0.0))
    (else
      (`MediaPlayer.Pause` (`self.video`)))))

(fn `UserConstructionScript`
  (`parent.UserConstructionScript`))